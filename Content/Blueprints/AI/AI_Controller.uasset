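; AI controller that makes its pawn track the ball along the Y axis, like a paddle opponent.
; On BeginPlay it caches the first BP_Ball found in the level and teleports the controlled pawn.
; Each Tick, FollowBall uses VInterpTo toward the ball and applies only the Y result, keeping X and Z fixed for smooth, lagging movement.
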(event EventBeginPlay
  (CallFunction|GetBall)
  (Transformation|SetActorLocationAndRotation (Pawn|GetControlledPawn) "0, 0, 0" "0, 0, 0" false true))

(event EventTick
  (params (DeltaSeconds :type Float%20%28single-precision%29))
  (CallFunction|FollowBall DeltaSeconds))

(fn ConstructionScript)

(fn FollowBall
  (params (DeltaTime :type Float%20%28single-precision%29))
  (bind _returnvalue (Pawn|GetControlledPawn))
  (bind _returnvalue_2 (Transformation|GetActorLocation _returnvalue))
  (Transformation|SetActorLocation _returnvalue (Math|Vector|MakeVector (.x _returnvalue_2) (.y (Math|Interpolation|VInterpTo (Math|Vector|MakeVector (.x _returnvalue_2) (.y _returnvalue_2) (.z _returnvalue_2)) (Transformation|GetActorLocation (Variables|Default|GetBall)) DeltaTime 2.0)) (.z _returnvalue_2)) false false))

(fn GetBall
  (bind _outactors (Actor|GetAllActorsOfClass "/Game/Blueprints/Ball/BP_Ball.BP_Ball_C"))
  (Variables|Default|SetBall (Utilities|Array|Get(acopy) _outactors)))